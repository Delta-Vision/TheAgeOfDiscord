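; Gate animator that moves a referenced actor along a spline when play begins and shows the battle start widget.
; BeginPlay calls OpenTheGate, which plays a half-speed timeline whose value samples the spline's world location by time.
; Each update sets the actor's transform with hard-coded rotation and scale, overriding its placed values.
; Despite the asset name, only opening is implemented.
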(event `OpenTheGate`
  (`/Engine/EditorBlueprintResources/StandardMacros.IsValid` (`self.ActorToAnimate`)
    (:`Is Valid`
      (`TimelineComponent.SetPlayRate` (`self.OpenGateTimeLine`) 0.5)
      (bind (_direction _time) (`Timeline|OpenGateTimeLine`)
        (:`Update`
          (`self.K2_SetActorTransform` (`self.ActorToAnimate`) (`KismetMathLibrary.MakeTransform` (`SplineComponent.GetLocationAtTime` (`self.Spline`) _time "World" false) (struct :`Yaw` 90.0) (1.6 1.5 1.5)) false false))))))

(event `self.ReceiveBeginPlay`
  (`self.OpenTheGate`)
  (bind _returnvalue (`|CreateWidget` "/Game/Widget_BattleStart.Widget_BattleStart_C"))
  (`/Engine/EditorBlueprintResources/StandardMacros.IsValid` _returnvalue
    (:`Is Valid`
      (`UserWidget.AddToViewport` _returnvalue 0))))

(event `self.ReceiveTick`
  (params (DeltaSeconds :type "Float (single-precision)")))

(fn `UserConstructionScript`)