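; Save component that persists a list of per-user stats entries in the "StatsSave" save slot.
; On BeginPlay its SERVER event loads the existing StatsSave object into SaveList, or creates a new one in memory if none exists.
; SaveID replaces the entry with a matching UserID or appends it, then writes the whole list to disk.
; LoadID searches the cached list by UserID and returns a found flag and the entry.
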(event `SERVER`
  (bind _returnvalue (`GameplayStatics.DoesSaveGameExist` "StatsSave"))
  (if _returnvalue
    (bind _returnvalue_2 (`GameplayStatics.LoadGameFromSlot` "StatsSave"))
    (bind _output_get (set `self.SaveGame` _returnvalue_2))
    (bind _asstats_save (cast `/Game/MarketPlace/CharacterStatsKit/Blueprints/StatsSave` _output_get))
    (set `self.SaveList` (`/Game/MarketPlace/CharacterStatsKit/Blueprints/StatsSave.Savelst` _asstats_save))
    (else
      (bind _returnvalue_3 (`GameplayStatics.CreateSaveGameObject` "/Game/MarketPlace/CharacterStatsKit/Blueprints/StatsSave.StatsSave_C"))
      (bind _output_get_2 (set `self.SaveGame` _returnvalue_3))
      (bind _asstats_save_2 (cast `/Game/MarketPlace/CharacterStatsKit/Blueprints/StatsSave` _output_get_2))
      (set `/Game/MarketPlace/CharacterStatsKit/Blueprints/StatsSave.Savelst` (`self.SaveList`) _asstats_save_2))))

(event `self.ReceiveBeginPlay`
  (`self.SERVER`))

(fn `LoadID`
  (params (ID :type Integer))
  (returns (bFound :type Boolean) (Item :type "/Game/MarketPlace/CharacterStatsKit/Blueprints/Structs/SaveStruct Structure"))
  (locals (FoundItem :type "/Game/MarketPlace/CharacterStatsKit/Blueprints/Structs/SaveStruct Structure" :default (struct :`UserID` -1 :`Class` "NewEnumerator0")) (Found :type Boolean))
  (for _array_element (`self.SaveList`)
    (if (== ID (`.UserID_3_E6E3AA2A42F6C1011EB592816CCFC7A8` (break `/Game/MarketPlace/CharacterStatsKit/Blueprints/Structs/SaveStruct` _array_element)))
      (set `local.FoundItem` _array_element)
      (set `local.Found` true)
      (break)))
  (return (`local.Found`) (`local.FoundItem`)))

(fn `SaveID`
  (params (ID :type Integer) (Item :type "/Game/MarketPlace/CharacterStatsKit/Blueprints/Structs/SaveStruct Structure (by ref)"))
  (locals (Found :type Boolean) (FoundItem :type "/Game/MarketPlace/CharacterStatsKit/Blueprints/Structs/SaveStruct Structure" :default (struct :`UserID` -1 :`Class` "NewEnumerator0")) (foundat :type Integer))
  (bind _savelist (`self.SaveList`))
  (bind _savegame (`self.SaveGame`))
  (for (_array_element _array_index) (`self.SaveList`)
    (if (== ID (`.UserID_3_E6E3AA2A42F6C1011EB592816CCFC7A8` (break `/Game/MarketPlace/CharacterStatsKit/Blueprints/Structs/SaveStruct` _array_element)))
      (set `local.FoundItem` _array_element)
      (set `local.Found` true)
      (set `local.foundat` _array_index)
      (break)))
  (if (`local.Found`)
    (`KismetArrayLibrary.Array_Set` _savelist (`local.foundat`) Item true)
    (else
      (`KismetArrayLibrary.Array_Add` (`self.SaveList`) Item)))
  (set `self.SaveList` _savelist)
  (bind _asstats_save (cast `/Game/MarketPlace/CharacterStatsKit/Blueprints/StatsSave` _savegame))
  (set `/Game/MarketPlace/CharacterStatsKit/Blueprints/StatsSave.Savelst` (`self.SaveList`) _asstats_save)
  (`GameplayStatics.SaveGameToSlot` _savegame "StatsSave"))